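; VR player arrow actor for the bow, grabbed and released through motion controller pickup events.
; Pickup, called by BP_MotionController, disables mesh physics, attaches the actor to the given component and plays a sound.
; Drop re-enables physics, detaches and immediately destroys the arrow.
; Hit, commented as projectile launch, briefly delays, then applies the actor's velocity as an impulse to Controllercollision at the actor's location.
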(event EventPickup
  (params (AttachTo :type Scene%20Component%20Object%20Reference))
  (bind _staticmesh (Variables|Default|GetStaticMesh))
  ;[1 1 1] grab
  (Physics|SetSimulatePhysics _staticmesh false)
  (Transformation|AttachComponentToComponent (VehicleSound|GetRootComponent) AttachTo "" "KeepWorld" "KeepWorld" "KeepWorld" true)
  (Audio|PlaySoundatLocation 0 (Transformation|GetWorldLocation _staticmesh) "0, 0, 0" 1.0 1.0 0.0 0 0 0))

(event Collision|EventHit
  (params (MyComp :type Primitive%20Component%20Object%20Reference) (Other :type Actor%20Object%20Reference) (OtherComp :type Primitive%20Component%20Object%20Reference) (bSelfMoved :type Boolean) (HitLocation :type Vector :default "0, 0, 0") (HitNormal :type Vector :default "0, 0, 0") (NormalImpulse :type Vector :default "0, 0, 0") (Hit :type Hit%20Result%20Structure%20%28by%20ref%29))
  ;[1 1 1] launch projectile
  (Utilities|FlowControl|Delay 0.01)
  (Physics|AddImpulseatLocation (Variables|Default|Getcontrollercollision) (Transformation|GetVelocity) (Transformation|GetActorLocation) "None"))

(event EventDrop
  ;[1 1 1] grab
  (Physics|SetSimulatePhysics (Variables|Default|GetStaticMesh) true)
  (Transformation|DetachFromActor "KeepWorld" "KeepWorld" "KeepWorld")
  (Actor|DestroyActor))

(fn ConstructionScript)