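; BP_SK_bow is a VR bow that attaches to a motion controller on pickup and regains physics when dropped.
; Each tick it shows the arrow while the right controller overlaps Pullposition, which follows that hand during a pull or resets to Pullstart.
; The arrow keeps aiming just above Bowholdposition.
; Right trigger press within the overlap starts the pull; release there spawns BP_playerarrowbp along the arrow's rotation, both with sound.
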(event EventPickup
  (params (AttachTo :type Scene%20Component%20Object%20Reference))
  ;[1 1 1] grab
  (bind _asmotion_controller_pawn (Utilities|Casting|CastToMotionControllerPawn (Game|Player|GetPlayerPawn 0)))
  (if (not (Collision|IsOverlappingActor (Variables|Default|GetPullposition) (Variables|/Game/VRreadybow/VirtualRealityBP/Blueprints/MotionControllerPawn.MotionControllerPawn_C|GetRightController _asmotion_controller_pawn) :!class /Script/Engine.PrimitiveComponent))
    (Physics|SetSimulatePhysics (Variables|Default|GetSkeletalMesh) false)
    (Transformation|AttachComponentToComponent (VehicleSound|GetRootComponent) AttachTo "" "SnapToTarget" "SnapToTarget" "SnapToTarget" true)))

(event EventDrop
  ;[1 1 1] grab
  (Physics|SetSimulatePhysics (Variables|Default|GetSkeletalMesh) true)
  (Transformation|DetachFromActor "KeepWorld" "KeepWorld" "KeepWorld"))

(event EventTick
  (params (DeltaSeconds :type Float%20%28single-precision%29))
  (bind _arrow (Variables|Default|GetArrow))
  (bind _bowholdposition (Variables|Default|GetBowholdposition))
  (bind _arrow_2 (Variables|Default|GetArrow))
  (bind _pullstart (Variables|Default|Getpullstart))
  (bind _returnvalue (Transformation|GetWorldTransform _pullstart))
  (bind _returnvalue_2 (Transformation|GetWorldLocation _bowholdposition))
  ;[1 1 1] arrow summon on overlap
  (Utilities|FlowControl|Sequence
    (:then_0
      (bind _asmotion_controller_pawn (Utilities|Casting|CastToMotionControllerPawn (Game|Player|GetPlayerPawn 0)))
      (if (Collision|IsOverlappingActor (Variables|Default|GetPullposition) (Variables|/Game/VRreadybow/VirtualRealityBP/Blueprints/MotionControllerPawn.MotionControllerPawn_C|GetRightController _asmotion_controller_pawn) :!class /Script/Engine.PrimitiveComponent)
        (Utilities|FlowControl|DoOnce false :!label _label
          (:Completed
            (Rendering|SetVisibility _arrow_2 true false)))
        (else
          (Rendering|SetVisibility _arrow_2 false false)
          (goto _label Reset))))
    (:then_1
      (if (Variables|Default|GetAttachtorighthand)
        (bind _asmotion_controller_pawn_2 (Utilities|Casting|CastToMotionControllerPawn (Game|Player|GetPlayerPawn 0)))
        (Transformation|SetWorldLocationAndRotation (Variables|Default|GetPullposition) (Math|Vector|MakeVector (.x (.location (Transformation|GetWorldTransform (Variables|/Game/VRreadybow/VirtualRealityBP/Blueprints/BP_MotionController.BP_MotionController_C|GetMotionController (Variables|/Game/VRreadybow/VirtualRealityBP/Blueprints/MotionControllerPawn.MotionControllerPawn_C|GetRightController _asmotion_controller_pawn_2))))) (.y (.location (Transformation|GetWorldTransform (Variables|/Game/VRreadybow/VirtualRealityBP/Blueprints/BP_MotionController.BP_MotionController_C|GetMotionController (Variables|/Game/VRreadybow/VirtualRealityBP/Blueprints/MotionControllerPawn.MotionControllerPawn_C|GetRightController _asmotion_controller_pawn_2))))) (.z (.location (Transformation|GetWorldTransform (Variables|/Game/VRreadybow/VirtualRealityBP/Blueprints/BP_MotionController.BP_MotionController_C|GetMotionController (Variables|/Game/VRreadybow/VirtualRealityBP/Blueprints/MotionControllerPawn.MotionControllerPawn_C|GetRightController _asmotion_controller_pawn_2)))))) "0, 0, 0" false false)
        (else
          ;;[1 1 1] arrow reset position
          (Transformation|SetWorldLocationAndRotation (Variables|Default|GetPullposition) (Math|Vector|MakeVector (.x (.location _returnvalue)) (.y (.location _returnvalue)) (.z (.location _returnvalue))) (Math|Rotator|MakeRotator (.roll (.rotation _returnvalue)) (.pitch (.rotation _returnvalue)) (.yaw (.rotation _returnvalue))) false false))))
    (:then_2
      ;;[1 1 1] arrow look position
      (Transformation|SetWorldRotation _arrow (Math|Rotator|FindLookatRotation (Transformation|GetWorldLocation _arrow) (Math|Vector|MakeVector (.x _returnvalue_2) (.y _returnvalue_2) (+ (.z _returnvalue_2) 5.0))) false false))))

(event Input|KeyboardEvents|MotionControllerRightTrigger
  (params (Key :type Key%20Structure))
  ;[1 1 1] grip button and spawn projectile
  (:Pressed
    (bind _asmotion_controller_pawn (Utilities|Casting|CastToMotionControllerPawn (Game|Player|GetPlayerPawn 0)))
    (if (Collision|IsOverlappingActor (Variables|Default|GetPullposition) (Variables|/Game/VRreadybow/VirtualRealityBP/Blueprints/MotionControllerPawn.MotionControllerPawn_C|GetRightController _asmotion_controller_pawn) :!class /Script/Engine.PrimitiveComponent)
      (Variables|Default|SetAttachtorighthand true)
      (Audio|PlaySoundatLocation 0 (Transformation|GetWorldLocation (Variables|Default|GetArrow)) "0, 0, 0" 3.0 1.0 0.0 0 0 0)))
  (:Released
    (bind _asmotion_controller_pawn_2 (Utilities|Casting|CastToMotionControllerPawn (Game|Player|GetPlayerPawn 0)))
    (if (Collision|IsOverlappingActor (Variables|Default|GetPullposition) (Variables|/Game/VRreadybow/VirtualRealityBP/Blueprints/MotionControllerPawn.MotionControllerPawn_C|GetRightController _asmotion_controller_pawn_2) :!class /Script/Engine.PrimitiveComponent)
      (Variables|Default|SetAttachtorighthand false)
      (Game|SpawnActorfromClass "/Game/VRreadybow/Bow/BP_playerarrowbp.BP_playerarrowbp_C" (Math|Transform|MakeTransform (Transformation|GetWorldLocation (Variables|Default|GetBowholdposition)) (Transformation|GetWorldRotation (Variables|Default|GetArrow)) "1,1,1") "AlwaysSpawn" 0 0)
      (Audio|PlaySoundatLocation 0 (Transformation|GetWorldLocation (Variables|Default|GetPullposition)) "0, 0, 0" 3.0 1.0 0.0 0 0 0))))

(fn ConstructionScript)