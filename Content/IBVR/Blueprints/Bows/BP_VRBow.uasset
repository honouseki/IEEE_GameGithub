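; Grabbable VR bow that attaches to a motion controller, mirrors for the left hand, and resets on drop, releasing any nocked arrow.
; A held arrow overlapping the pull point becomes nocked, and its hand, or a secondary grip, drives the string.
; Tick moves the pull point with that hand, aims the arrow toward the hand-dependent rest, stores draw length as potential energy, and plays a sound past a draw threshold.
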(event OnComponentBeginOverlap(BowPullPoint)
  (params (OverlappedComponent :type Primitive%20Component%20Object%20Reference) (OtherActor :type Actor%20Object%20Reference) (OtherComp :type Primitive%20Component%20Object%20Reference) (OtherBodyIndex :type Integer) (bFromSweep :type Boolean) (SweepResult :type Hit%20Result%20Structure%20%28by%20ref%29))
  ;[1 1 1] Start positioning the held arrow, and pull string
  (bind _asbp_base_arrow (Utilities|Casting|CastToBP_BaseArrow OtherActor))
  (bind _held (Default|Held _asbp_base_arrow))
  (if (and _held (Variables|Default|GetbPickedUp))
    (Variables|Default|SetbPullingString true)
    (bind _hand (Default|GetHand _asbp_base_arrow))
    (Transformation|DetachFromActor _asbp_base_arrow "KeepRelative" "KeepRelative" "KeepWorld")
    (Variables|Bow|SetStringHand _hand)
    (bind _output_get (Variables|Bow|SetKnockedArrow _asbp_base_arrow))
    (Variables|/Game/IBVR/Blueprints/Arrows/BP_BaseArrow.BP_BaseArrow_C|SetGripType _output_get "NewEnumerator4")
    (Variables|/Game/IBVR/Blueprints/Arrows/BP_BaseArrow.BP_BaseArrow_C|SetAssociatedBow _asbp_base_arrow self)
    (Variables|/Game/IBVR/Blueprints/Arrows/BP_BaseArrow.BP_BaseArrow_C|SetbKnocked _output_get true)))

(event Custom|ReleaseArrowRef
  (Variables|Default|SetbPullingString false)
  (Variables|Bow|SetKnockedArrow 0)
  (Variables|Bow|SetStringHand 0))

(event EventPickup
  (params (AttachTo :type Scene%20Component%20Object%20Reference))
  ;[1 1 1] Picked up and Dropped
  (Physics|SetSimulatePhysics (Variables|Default|GetBow) false)
  (Transformation|AttachComponentToComponent AttachTo "None" "SnapToTarget" "SnapToTarget" "SnapToTarget" false)
  (Transformation|SetActorRelativeLocation (Variables|Bow|GetAttachOffset))
  (Variables|Default|SetbPickedUp true)
  (bind _asbp_ibmotion_controller (Utilities|Casting|CastToBP_IBMotionController (Components|GetOwner AttachTo)))
  (switch Utilities|FlowControl|Switch|SwitchonEControllerHand (Variables|/Game/IBVR/Blueprints/BP_IBMotionController.BP_IBMotionController_C|GetHand _asbp_ibmotion_controller)
    (:Left
      (Transformation|SetActorScale3D "1.000000,-1.000000,1.000000"))
    (:Right
      (Transformation|SetActorScale3D "1.000000,1.000000,1.000000"))))

(event EventTick
  (params (DeltaSeconds :type Float%20%28single-precision%29))
  (bind _knockedarrow (Variables|Bow|GetKnockedArrow))
  (bind _stringhand (Variables|Bow|GetStringHand))
  (bind _bowpullpoint (Variables|Default|GetBowPullPoint))
  ;[1 1 1] String Location and Animation
  (Utilities|FlowControl|Sequence
    (:then_0
      (Variables|Bow|SetHandPullLocation (Transformation|GetWorldLocation (Variables|Default|GetBowPullPoint)))
      (if (Variables|Default|GetbPullingString)
        (Utilities|IsValid _stringhand
          (:Is%20Valid
            (Transformation|SetWorldLocation _bowpullpoint (+ (Transformation|GetWorldLocation (Variables|/Game/IBVR/Blueprints/BP_IBMotionController.BP_IBMotionController_C|GetMotionController _stringhand)) (* (Math|Vector|GetForwardVector _bowpullpoint) 4.0)) false false)))
        (else
          (Transformation|SetRelativeLocation (Variables|Default|GetBowPullPoint) (Variables|Bow|GetDefaultBowStringPoint) false false))))
    (:then_1
      (Utilities|IsValid _knockedarrow
        (:Is%20Valid
          (if (Variables|/Game/IBVR/Blueprints/Arrows/BP_BaseArrow.BP_BaseArrow_C|GetbGrabbed _knockedarrow)
            (CallFunction|CheckArrowLimits)
            (CallFunction|PositionArrow (Variables|Bow|GetKnockedArrow))))))))

(event EventSecondRelease
  ;[1 1 1] Release Secondary Grip
  (Variables|Default|SetbPullingString false)
  (Variables|Bow|SetStringHand 0))

(event EventDrop
  ;[1 1 1] Picked up and Dropped
  (Transformation|SetActorScale3D "1.000000,1.000000,1.000000")
  (Utilities|IsValid (Variables|Bow|GetKnockedArrow)
    (:Is%20Valid
      (Variables|/Game/IBVR/Blueprints/Arrows/BP_BaseArrow.BP_BaseArrow_C|SetbKnocked (Variables|Bow|GetKnockedArrow) false)
      (Default|ManualDrop (Variables|Bow|GetKnockedArrow))
      (Variables|Bow|SetKnockedArrow 0)
      (if (Utilities|IsValid (Variables|/Game/IBVR/Blueprints/Arrows/BP_BaseArrow.BP_BaseArrow_C|GetHandHolding (Variables|Bow|GetKnockedArrow)))
        (Variables|/Game/IBVR/Blueprints/BP_IBMotionController.BP_IBMotionController_C|SetGripState (Variables|/Game/IBVR/Blueprints/Arrows/BP_BaseArrow.BP_BaseArrow_C|GetHandHolding (Variables|Bow|GetKnockedArrow)) "NewEnumerator0")))
    (:Is%20Not%20Valid
      _))
  (Transformation|DetachFromActor "KeepWorld" "KeepWorld" "KeepWorld")
  (Physics|SetSimulatePhysics (Variables|Default|GetBow) (Variables|Bow|GetUsePhysics))
  (Variables|Bow|SetHandPullLocation (Variables|Bow|GetDefaultBowStringPoint))
  (Variables|Default|SetbPickedUp false)
  (Variables|Default|SetbPullingString false)
  (Variables|Bow|SetStringHand 0))

(event EventSecondGrab
  (params (Hand :type BP%20IB%20Motion%20Controller%20Object%20Reference))
  ;[1 1 1] Begin Secondary Grip
  (Variables|Default|SetbPullingString true)
  (Variables|Bow|SetStringHand Hand))

(event EventBeginPlay
  (Physics|SetSimulatePhysics (Variables|Default|GetBow) (and (Variables|Bow|GetStartSimulatingPhysics) (Variables|Bow|GetUsePhysics))))

(fn ConstructionScript
  (Variables|Bow|SetHandPullLocation (Transformation|GetWorldLocation (Variables|Default|GetBowPullPoint))))

(fn PositionArrow
  (params (Arrow :type BP%20Base%20Arrow%20Object%20Reference))
  (bind _knockedarrow (Variables|Bow|GetKnockedArrow))
  (bind _hand (Default|GetHand Arrow))
  (bind _output_get (Variables|Default|SetLength (Math|Vector|VectorLength (- (Transformation|GetWorldLocation (Variables|Default|GetPullStartPoint)) (Variables|Bow|GetHandPullLocation)))))
  (Variables|/Game/IBVR/Blueprints/Arrows/BP_BaseArrow.BP_BaseArrow_C|SetPotentialEnergy _knockedarrow _output_get)
  (Transformation|SetActorTransform _knockedarrow (Math|Transform|MakeTransform (+ (Variables|Bow|GetHandPullLocation) (Math|Vector|Normalize (- (select (Variables|Default|GetBowFlipped) (|KnockSide_2 (Transformation|GetWorldLocation (Variables|Default|GetKnockLeft)) (Transformation|GetWorldLocation (Variables|Default|GetKnockLeft)) (Variables|/Game/IBVR/Blueprints/BP_IBMotionController.BP_IBMotionController_C|GetHand _hand)) (|KnockSide (Transformation|GetWorldLocation (Variables|Default|GetKnockLeft)) (Transformation|GetWorldLocation (Variables|Default|GetKnockRight)) (Variables|/Game/IBVR/Blueprints/BP_IBMotionController.BP_IBMotionController_C|GetHand _hand))) (Variables|Bow|GetHandPullLocation)))) (Math|Rotator|MakeRotfromX (- (select (Variables|Default|GetBowFlipped) (|KnockSide_2 (Transformation|GetWorldLocation (Variables|Default|GetKnockLeft)) (Transformation|GetWorldLocation (Variables|Default|GetKnockLeft)) (Variables|/Game/IBVR/Blueprints/BP_IBMotionController.BP_IBMotionController_C|GetHand _hand)) (|KnockSide (Transformation|GetWorldLocation (Variables|Default|GetKnockLeft)) (Transformation|GetWorldLocation (Variables|Default|GetKnockRight)) (Variables|/Game/IBVR/Blueprints/BP_IBMotionController.BP_IBMotionController_C|GetHand _hand))) (Variables|Bow|GetHandPullLocation))))))

(fn CheckArrowLimits
  (if (< (.x (Variables|/Script/Engine.SceneComponent|GetRelativeLocation (Variables|Default|GetBowPullPoint))) -38.0)
    (if (Variables|Default|GetbPlayedPullSound)
      (return)
      (else
        (Development|PrintString "PULL!")
        (Variables|Default|SetbPlayedPullSound true)
        (Audio|PlaySoundatLocation "/Game/IBVR/Sounds/Cues/Bow_Pull_Cue.Bow_Pull_Cue" (Transformation|GetActorLocation))
        (return)))
    (else
      (Variables|Default|SetbPlayedPullSound false)
      (return))))

(fn GetHand
  (return 0))

(fn GrabType
  (return "NewEnumerator2"))

(fn Held
  (return (Variables|Default|GetbPickedUp)))