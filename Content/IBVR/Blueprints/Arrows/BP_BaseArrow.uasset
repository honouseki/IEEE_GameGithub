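; Base VR arrow actor that can be picked up by a motion controller, knocked on a bow and fired.
; Pickup attaches it with a hand-mirrored offset; dropping either restores physics or, when knocked, launches it and releases the bow's reference.
; In flight, Tick moves it manually at a speed scaled from PotentialEnergy.
; A box trace at the tip, ignoring bows, stops it on impact, embedding it with sound and hit effects.
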(event Custom|ManualDrop
  ;[1 1 1] Picked up and Dropped
  (Transformation|DetachFromActor "KeepWorld" "KeepWorld" "KeepWorld")
  (if (not (Variables|Arrow|GetbKnocked))
    (Physics|SetSimulatePhysics (Variables|Default|GetArrow) (Variables|Arrow|GetUsePhysics))
    (Variables|Arrow|SetHandHolding 0)
    (Variables|Arrow|SetbGrabbed false)
    (else
      (Audio|PlaySoundatLocation "/Game/IBVR/Sounds/Cues/ReleaseArrow_Cue.ReleaseArrow_Cue" (Transformation|GetActorLocation))
      ;[1 1 1] If knocked set speed and traveling
      (Components|Activation|Activate (Variables|Default|GetP_ArrowTrail) true)
      (Default|ReleaseArrowRef (Variables|Arrow|GetAssociatedBow))
      (Variables|Arrow|SetbTraveling true)
      (Variables|Arrow|SetAssociatedBow 0)
      (Variables|Default|SetGripType "NewEnumerator3")
      (Variables|Arrow|SetHandHolding 0)
      (Variables|Arrow|SetbGrabbed false)
      (Variables|Arrow|SetbKnocked false))))

(event EventPickup
  (params (AttachTo :type Scene%20Component%20Object%20Reference))
  (bind _attachoffset (Variables|Arrow|GetAttachOffset))
  (bind (_x _y _z) (Math|Vector|BreakVector _attachoffset))
  ;[1 1 1] Picked up and Dropped
  (Physics|SetSimulatePhysics (Variables|Default|GetArrow) false)
  (Transformation|AttachComponentToComponent AttachTo "None" "SnapToTarget" "SnapToTarget" "SnapToTarget" false)
  (bind _asbp_ibmotion_controller (Utilities|Casting|CastToBP_IBMotionController (Components|GetOwner AttachTo)))
  (Variables|Arrow|SetHandHolding _asbp_ibmotion_controller)
  (Variables|Arrow|SetbGrabbed true)
  (switch Utilities|FlowControl|Switch|SwitchonEControllerHand (Variables|/Script/HeadMountedDisplay.MotionControllerComponent|GetHand (Variables|/Game/IBVR/Blueprints/BP_IBMotionController.BP_IBMotionController_C|GetMotionController _asbp_ibmotion_controller))
    (:Left
      (Transformation|SetActorRelativeLocation (Variables|Arrow|GetAttachOffset)))
    (:Right
      (Transformation|SetActorRelativeLocation (Math|Vector|MakeVector _x (* _y -1.0) _z)))))

(event EventDrop
  ;[1 1 1] Picked up and Dropped
  (Transformation|DetachFromActor "KeepWorld" "KeepWorld" "KeepWorld")
  (if (not (Variables|Arrow|GetbKnocked))
    (Physics|SetSimulatePhysics (Variables|Default|GetArrow) (Variables|Arrow|GetUsePhysics))
    (Variables|Arrow|SetHandHolding 0)
    (Variables|Arrow|SetbGrabbed false)
    (else
      (Audio|PlaySoundatLocation "/Game/IBVR/Sounds/Cues/ReleaseArrow_Cue.ReleaseArrow_Cue" (Transformation|GetActorLocation))
      ;[1 1 1] If knocked set speed and traveling
      (Components|Activation|Activate (Variables|Default|GetP_ArrowTrail) true)
      (Default|ReleaseArrowRef (Variables|Arrow|GetAssociatedBow))
      (Variables|Arrow|SetbTraveling true)
      (Variables|Arrow|SetAssociatedBow 0)
      (Variables|Default|SetGripType "NewEnumerator3")
      (Variables|Arrow|SetHandHolding 0)
      (Variables|Arrow|SetbGrabbed false)
      (Variables|Arrow|SetbKnocked false))))

(event EventTick
  (params (DeltaSeconds :type Float%20%28single-precision%29))
  (bind _arrowtip (Variables|Default|GetArrowTip))
  (bind _returnvalue (Transformation|GetWorldLocation _arrowtip))
  ;[1 1 1] Calculate arrow speed and direction
  (if (Variables|Arrow|GetbTraveling)
    (bind (_newlocation _transform) (CallFunction|CalcSpeedGravity (* (Variables|Arrow|GetPotentialEnergy) 5e+01)))
    (Development|PrintString (Utilities|String|ToString(Vector) (Math|Vector|GetUnitDirection(Vector) (Transformation|GetActorLocation) _newlocation)) false false)
    (Transformation|SetActorTransform _transform)
    ;[1 1 1] Hit Something
    (bind _outhit (Collision|BoxTraceByChannel _returnvalue _returnvalue "5.000000,5.000000,5.000000" (Transformation|GetActorRotation) "TraceTypeQuery1" false (Variables|Default|GetIgnoredActors) "None"))
    (bind _output_get (Variables|Arrow|SetbTraveling (not (.bBlockingHit (Collision|BreakHitResult _outhit)))))
    (if (not _output_get)
      (Transformation|SetActorLocation (+ (Transformation|GetActorLocation) (* (Math|Vector|GetForwardVector (Transformation|GetActorRotation)) (Variables|Default|GetPenetrationDepth))) false false)
      (Components|Activation|Deactivate (Variables|Default|GetP_ArrowTrail))
      (Audio|PlaySoundatLocation "/Game/IBVR/Sounds/Cues/ArrowHit_Cue.ArrowHit_Cue" (Transformation|GetActorLocation))
      (Components|Activation|Activate (Variables|Default|GetP_HitMarker) true))))

(event EventBeginPlay
  (Physics|SetSimulatePhysics (Variables|Default|GetArrow) (and (Variables|Arrow|GetStartSimulatingPhysics) (Variables|Arrow|GetUsePhysics)))
  (bind _outactors (Actor|GetAllActorsOfClass "/Game/IBVR/Blueprints/Bows/BP_VRBow.BP_VRBow_C"))
  (Variables|Default|SetIgnoredActors _outactors))

(fn ConstructionScript)

(fn CalcSpeedGravity
  (params (ReleaseSpeed :type Float%20%28single-precision%29))
  (bind _returnvalue (Transformation|GetActorForwardVector))
  (bind _returnvalue_2 (Utilities|Time|GetWorldDeltaSeconds))
  (bind _deltalocation (Utilities|ForwardVelocity _returnvalue _returnvalue_2 ReleaseSpeed))
  (bind (_location _rotation _scale) (Math|Transform|BreakTransform _deltalocation))
  (return _location (Math|Transform|MakeTransform _location _rotation _scale)))

(fn GetHand
  (return (Variables|Arrow|GetHandHolding)))

(fn GrabType
  (return (Variables|Default|GetGripType)))

(fn Held
  (return (Variables|Arrow|GetbGrabbed)))