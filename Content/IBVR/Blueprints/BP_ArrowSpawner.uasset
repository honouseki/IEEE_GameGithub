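; BP_ArrowSpawner is a grabbable VR dispenser that gives the motion controller a new arrow when picked up.
; On BeginPlay it sets its static mesh to match the configured arrow class.
; Pickup disables its collision, spawns that arrow at the mesh's transform, then after a brief delay has the controller call GrabActor and restores collision.
; The spawner never reports itself as held.
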(event EventBeginPlay
  (bind _staticmesh (Variables|Default|GetStaticMesh))
  (Utilities|FlowControl|Sequence
    (:then_0
      (if (== (Variables|Default|GetArrowToSpawn) "/Game/IBVR/Blueprints/Arrows/BP_Arrow1.BP_Arrow1_C")
        (Components|StaticMesh|SetStaticMesh _staticmesh "/Game/IBVR/Meshes/Arrows/SM_Arrow2.SM_Arrow2")))
    (:then_1
      (if (== (Variables|Default|GetArrowToSpawn) "/Game/IBVR/Blueprints/Arrows/BP_Arrow2.BP_Arrow2_C")
        (Components|StaticMesh|SetStaticMesh _staticmesh "/Game/IBVR/Meshes/Arrows/SM_Arrow1.SM_Arrow1")))
    (:then_2
      (if (== (Variables|Default|GetArrowToSpawn) "/Game/IBVR/Blueprints/Arrows/BP_HomemadeArrow.BP_HomemadeArrow_C")
        (Components|StaticMesh|SetStaticMesh _staticmesh "/Game/IBVR/Meshes/Arrows/HomemadeArrow.HomemadeArrow")))))

(event EventPickup
  (params (AttachTo :type Scene%20Component%20Object%20Reference))
  (bind _returnvalue (Components|GetOwner AttachTo))
  (Collision|SetActorEnableCollision false)
  (Game|SpawnActorfromClass (Variables|Default|GetArrowToSpawn) (Transformation|GetWorldTransform (Variables|Default|GetStaticMesh)) "AlwaysSpawn" _returnvalue 0)
  (bind _asbp_ibmotion_controller (Utilities|Casting|CastToBP_IBMotionController _returnvalue))
  (Utilities|FlowControl|Delay 0.07)
  (Default|GrabActor _asbp_ibmotion_controller)
  (Collision|SetActorEnableCollision true))

(fn ConstructionScript)

(fn GetHand
  (return 0))

(fn GrabType
  (return "NewEnumerator0"))

(fn Held
  (return false))